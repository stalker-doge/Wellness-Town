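; Base NPC Blueprint that caches the player character on BeginPlay and holds scaffolding for proximity interaction and dialogue UI.
; InRange and OnRangeExited are empty; the code to create and destroy a screen-space interaction widget on the capsule is disconnected.
; DialogueSetUp adds a screen-space TestDialogue widget component above the NPC, but only when the Widget variable is already valid, and nothing here calls it.
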(event EventBeginPlay
  (bind _asbp_player_character (Utilities|Casting|CastToBP_PlayerCharacter (Game|GetPlayerCharacter 0)))
  (Variables|Default|SetPlayerCharacter _asbp_player_character))

(event EventInRange
  (params (Player :type BP%20Player%20Character%20Object%20Reference)))

(event EventOnRangeExited)

(fn ConstructionScript)

(fn DialogueSetUp
  (params (Player :type BP%20Player%20Character%20Object%20Reference))
  (Variables|Default|GetWidget
    (:then
      (bind _returnvalue (UserInterface|CreateWidget "/Game/DEV/Ben_S/UI/InGame/testDialogue.testDialogue_C" (.AsWTPlayer%20Controller (Utilities|Casting|CastToWTPlayerController (Pawn|GetController Player)))))
      (bind _returnvalue_2 (AddComponent|AddWidgetComponent false (Math|Transform|MakeTransform "0.000000,0.000000,200.000000" "0, 0, 0" "1.000000,1.000000,1.000000")))
      (bind _output_get (Variables|Default|SetWidget _returnvalue_2))
      (UserInterface|SetWidget _output_get _returnvalue)
      (Class|WidgetComponent|SetWidgetSpace _output_get "Screen")
      (Class|WidgetComponent|SetDrawatDesiredSize _output_get true)
      (Collision|SetCollisionEnabled _output_get "QueryOnly"))
    (:else)))