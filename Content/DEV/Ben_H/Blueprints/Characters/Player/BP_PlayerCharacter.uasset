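; Player character Blueprint with a draft interaction system built around an interact collider and the I_Interact interface.
; Disconnected logic would send OnInteractMessage to overlapping actors implementing the interface, and range enter and exit messages.
; The Interact input and both collider overlap events are empty, so none of that logic runs.
; The construction script is empty.
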(event OnComponentBeginOverlap(_interactCollider)
  (params (OverlappedComponent :type Primitive%20Component%20Object%20Reference) (OtherActor :type Actor%20Object%20Reference) (OtherComp :type Primitive%20Component%20Object%20Reference) (OtherBodyIndex :type Integer) (bFromSweep :type Boolean) (SweepResult :type Hit%20Result%20Structure%20%28by%20ref%29)))

(event OnComponentEndOverlap(_interactCollider)
  (params (OverlappedComponent :type Primitive%20Component%20Object%20Reference) (OtherActor :type Actor%20Object%20Reference) (OtherComp :type Primitive%20Component%20Object%20Reference) (OtherBodyIndex :type Integer)))

(event Input|EnhancedActionEvents|EnhancedInputActionInteract
  (params (ActionValue :type Boolean) (ElapsedSeconds :type Float%20%28double-precision%29) (TriggeredSeconds :type Float%20%28double-precision%29) (InputAction :type Input%20Action%20Object%20Reference :default "/Game/DEV/Ben_H/Blueprints/Input/Interact.Interact")))

(fn ConstructionScript)