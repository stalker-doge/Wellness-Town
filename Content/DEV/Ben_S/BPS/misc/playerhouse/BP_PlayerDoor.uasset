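; BP_PlayerDoor is an interactable player house door that swings open and then loads another level.
; When a player comes in range it adds a screen-space W_Interaction prompt as a runtime widget component, which it destroys when the range is exited.
; Interacting plays the DoorRotate timeline to yaw the door mesh open, and the timeline's completion opens the level referenced by OpenLevel.
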(event EventInRange
  (params (Player :type BP%20Player%20Character%20Object%20Reference))
  (Variables|Default|Getwidget
    (:then)
    (:else
      (bind _returnvalue (UserInterface|CreateWidget "/Game/DEV/Ben_S/UI/InGame/W_Interaction.W_Interaction_C" (.AsWTPlayer%20Controller (Utilities|Casting|CastToWTPlayerController (Pawn|GetController Player)))))
      (bind _returnvalue_2 (AddComponent|AddWidgetComponent false))
      (bind _output_get (Variables|Default|Setwidget _returnvalue_2))
      (UserInterface|SetWidget _output_get _returnvalue)
      (Class|WidgetComponent|SetWidgetSpace _output_get "Screen")
      (Class|WidgetComponent|SetDrawatDesiredSize _output_get true)
      (Collision|SetCollisionEnabled _output_get "QueryOnly"))))

(event EventOnRangeExited
  (bind _widget (Variables|Default|Getwidget)
    (:then
      (Components|DestroyComponent _widget))
    (:else)))

(event EventOnInteract
  (params (Player :type BP%20Player%20Character%20Object%20Reference))
  (bind _rotatedoor (Timeline|DoorRotate Play)
    (:Update
      (Transformation|SetRelativeRotation (Variables|Default|GetPlayer_House_Door) (Math|Rotator|MakeRotator 0.0 0.0 (Math|Float|Lerp 0.0 8e+01 _rotatedoor)) false false))
    (:Finished
      (Game|OpenLevel(byObjectReference) "/Game/DEV/Ben_K/MAPS/OpenLevel.OpenLevel"))))

(fn ConstructionScript)