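; BP_FishingCam is a development interactable that toggles a player's fishing state.
; Entering range swaps the Cube to a highlight test material and spawns a screen-space W_Interaction prompt in a runtime-added widget component.
; Leaving range restores the other material and destroys that component.
; Interacting alternates the player's IsFishing flag through a FlipFlop, so the toggle follows this actor's own state rather than the player's current value.
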(event EventInRange
  (params (Player :type BP%20Player%20Character%20Object%20Reference))
  (Rendering|Material|SetMaterial (Variables|Default|GetCube) 0 "/Game/DEV/Ben_S/Mats/M_testTranslucent1.M_testTranslucent1")
  (Variables|Default|Getwidget
    (:then)
    (:else
      (bind _returnvalue (UserInterface|CreateWidget "/Game/DEV/Ben_S/UI/InGame/W_Interaction.W_Interaction_C" (.AsWTPlayer%20Controller (Utilities|Casting|CastToWTPlayerController (Pawn|GetController Player)))))
      (bind _returnvalue_2 (AddComponent|AddWidgetComponent false))
      (bind _output_get (Variables|Default|Setwidget _returnvalue_2))
      (UserInterface|SetWidget _output_get _returnvalue)
      (Class|WidgetComponent|SetWidgetSpace _output_get "Screen")
      (Class|WidgetComponent|SetDrawatDesiredSize _output_get true)
      (Collision|SetCollisionEnabled _output_get "QueryOnly"))))

(event EventOnRangeExited
  (Rendering|Material|SetMaterial (Variables|Default|GetCube) 0 "/Game/DEV/Ben_S/Mats/M_testTranslucent.M_testTranslucent")
  (bind _widget (Variables|Default|Getwidget)
    (:then
      (Components|DestroyComponent _widget))
    (:else)))

(event EventOnInteract
  (params (Player :type BP%20Player%20Character%20Object%20Reference))
  (Utilities|FlowControl|FlipFlop
    (:A
      (Variables|/Game/DEV/Ben_H/Blueprints/Characters/Player/BP_PlayerCharacter.BP_PlayerCharacter_C|SetIsFishing Player true))
    (:B
      (Variables|/Game/DEV/Ben_H/Blueprints/Characters/Player/BP_PlayerCharacter.BP_PlayerCharacter_C|SetIsFishing Player false))))

(fn ConstructionScript)