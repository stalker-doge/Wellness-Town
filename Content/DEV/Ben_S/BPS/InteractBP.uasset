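; InteractBP is an interactable that shows an interaction prompt when a player is in range and has hooks for quests.
; BeginPlay caches the character's AC_Questlog component.
; InRange creates a screen-space W_Interaction widget component at runtime if none exists, and OnRangeExited destroys it.
; QuestInteract returns the fixed identifier "Bin", while IfStage compares an index to the first stage's number without producing a result.
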(event EventInRange
  (params (Player :type Player%20Character%20Object%20Reference))
  (Variables|Default|Getwidget
    (:then)
    (:else
      (bind _returnvalue (UserInterface|CreateWidget "/Game/DEV/Ben_S/UI/InGame/W_Interaction.W_Interaction_C" (.AsWTPlayer%20Controller (Utilities|Casting|CastToWTPlayerController (Pawn|GetController Player)))))
      (bind _returnvalue_2 (AddComponent|AddWidgetComponent false))
      (bind _output_get (Variables|Default|Setwidget _returnvalue_2))
      (UserInterface|SetWidget _output_get _returnvalue)
      (Class|WidgetComponent|SetWidgetSpace _output_get "Screen")
      (Class|WidgetComponent|SetDrawatDesiredSize _output_get true)
      (Collision|SetCollisionEnabled _output_get "QueryOnly"))))

(event EventOnRangeExited
  (bind _widget (Variables|Default|Getwidget)
    (:then
      (Components|DestroyComponent _widget))
    (:else)))

(event EventBeginPlay
  (bind _player (CallFunction|GetCharacterBP))
  (bind _returnvalue (Actor|GetComponentbyClass _player "/Game/DEV/Ben_S/BPS/Quest/AC_Questlog.AC_Questlog_C"))
  (Utilities|IsValid _returnvalue
    (:Is%20Valid
      (Variables|Default|SetQuestLog _returnvalue))))

(fn ConstructionScript)

(fn IfStage
  (params (Index :type Integer))
  (if (== (.StageNumber (Utilities|Struct|BreakDS_QuestStageDetails (Utilities|Array|Get(acopy) (.stage (Variables|Default|GetStage))))) Index)
    (return)))

(fn QuestInteract
  (return "Bin"))