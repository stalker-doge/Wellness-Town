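; Quest giver component that offers one data-table quest to the player and handles its turn-in.
; DisplayQuest looks up the QuestData row and shows it in a W_Quest widget.
; GiveQuest adds the passed quest ID to the character's ACQuestlog if the QuestData quest is neither active nor completed.
; QuestInteract completes a finished, not-yet-turned-in quest, returning the owner's display name then or when the quest is still untaken.
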(event EventBeginPlay)

(event EventTick
  (params (DeltaSeconds :type Float%20%28single-precision%29)))

(fn DisplayQuest
  (bind _questdata (Variables|Default|GetQuestData))
  (bind _returnvalue (Utilities|GetDataTableRow (.datatable _questdata) (.rowname _questdata))
    (:then
      (bind _output_get (Variables|Default|SetQuest%20Data%20Row%20Name (.rowname _questdata)))
      (bind _returnvalue_2 (UserInterface|CreateWidget "/Game/DEV/Ben_S/UI/InGame/Quest/W_Quest.W_Quest_C" 0 _returnvalue _output_get))
      (UserInterface|Viewport|AddtoViewport _returnvalue_2 0))))

(fn GiveQuest
  (params (QuestID :type Name))
  (bind _player (CallFunction|GetCharacterBP))
  (bind _questdata (Variables|Default|GetQuestData))
  (bind _ac_questlog (Variables|/Game/DEV/Ben_H/Blueprints/Characters/Player/BP_PlayerCharacter.BP_PlayerCharacter_C|GetAC_Questlog _player))
  (if (and (not (Default|QueryActiveQuest _ac_questlog (.rowname _questdata))) (not (.ReturnValue (Default|QueryCompletedQuests _ac_questlog (.rowname _questdata)))))
    (Default|AddNewQuest (Variables|/Game/DEV/Ben_H/Blueprints/Characters/Player/BP_PlayerCharacter.BP_PlayerCharacter_C|GetAC_Questlog (CallFunction|GetCharacterBP)) QuestID)))

(fn QuestInteract
  (bind _player (CallFunction|GetCharacterBP))
  (bind _returnvalue (Components|GetOwner))
  (bind _player_2 (CallFunction|GetCharacterBP))
  (bind _questdata (Variables|Default|GetQuestData))
  (bind _questdata_2 (Variables|Default|GetQuestData))
  (bind _returnvalue_2 (Utilities|GetDisplayName _returnvalue))
  (bind _ac_questlog (Variables|/Game/DEV/Ben_H/Blueprints/Characters/Player/BP_PlayerCharacter.BP_PlayerCharacter_C|GetAC_Questlog _player))
  (bind _ac_questlog_2 (Variables|/Game/DEV/Ben_H/Blueprints/Characters/Player/BP_PlayerCharacter.BP_PlayerCharacter_C|GetAC_Questlog _player_2))
  (if (and (not (Default|QueryActiveQuest _ac_questlog (.rowname _questdata_2))) (not (.ReturnValue (Default|QueryCompletedQuests _ac_questlog (.rowname _questdata_2)))))
    (return _returnvalue_2)
    (else
      (bind _array_element (Default|GetQuestActor _ac_questlog_2 (.rowname _questdata)))
      (if (and (Variables|/Game/DEV/Ben_S/BPS/Quest/QuestBP.QuestBP_C|GetIsComplete _array_element) (not (Variables|/Game/DEV/Ben_S/BPS/Quest/QuestBP.QuestBP_C|GetIsTurnedIn _array_element)))
        (Default|CompleteQuest _ac_questlog_2 (.rowname _questdata))
        (return _returnvalue_2)))))