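; Quest log component that adds, tracks, completes and answers queries on quests by ID.
; Each new quest records its ID as active and spawns a QuestBP actor that holds its state.
; Completion moves the ID to the completed list, flags the actor as turned in and fires OnQuestCompleted.
; Tracking reuses one on-screen W_QuestTracker widget, and completion queries report turned in when no quest actor exists.
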(fn AddNewQuest
  (params (QuestID :type Name))
  (Utilities|Array|AddUnique (Variables|Default|GetCurrentActiveQuests) QuestID)
  (bind _returnvalue (Game|SpawnActorfromClass "/Game/DEV/Ben_S/BPS/Quest/QuestBP.QuestBP_C" (Math|Transform|MakeTransform "0, 0, 0" "0, 0, 0" "1.000000,1.000000,1.000000") "Undefined" "MultiplyWithRoot" 0 QuestID 0))
  (Utilities|Array|Add (Variables|Default|GetCurrentQuests) _returnvalue)
  (return _returnvalue))

(fn CompleteQuest
  (params (QuestID :type Name%20%28by%20ref%29))
  (Utilities|Array|AddUnique (Variables|Default|GetCompletedQuests) QuestID)
  (Utilities|Array|RemoveItem (Variables|Default|GetCurrentActiveQuests) QuestID)
  (bind _array_element (CallFunction|GetQuestActor QuestID))
  (Variables|/Game/DEV/Ben_S/BPS/Quest/QuestBP.QuestBP_C|SetIsTurnedIn _array_element true)
  (Default|CallOnQuestCompleted _array_element))

(fn QueryActiveQuest
  (params (QuestID :type Name))
  (return (Utilities|Array|ContainsItem (Variables|Default|GetCurrentActiveQuests) QuestID)))

(fn TrackQuest
  (params (QuestActor :type Quest%20BP%20Object%20Reference))
  (Variables|Default|GetTracker
    (:then
      (Default|Update (Variables|Default|GetTracker) QuestActor))
    (:else
      (bind _returnvalue (UserInterface|CreateWidget "/Game/DEV/Ben_S/UI/InGame/Quest/W_QuestTracker.W_QuestTracker_C" 0 QuestActor))
      (bind _output_get (Variables|Default|SetTracker _returnvalue))
      (UserInterface|Viewport|AddtoViewport _output_get -1))))

(fn GetQuestActor
  (params (QuestID :type Name))
  (for _array_element (Variables|Default|GetCurrentQuests)
    (if (== (Variables|/Game/DEV/Ben_S/BPS/Quest/QuestBP.QuestBP_C|GetQuestID _array_element) QuestID)
      (return _array_element))))

(fn QueryCompletedQuests
  (params (QuestID :type Name))
  (bind _completedquests (Variables|Default|GetCompletedQuests))
  (bind _returnvalue (Utilities|Array|ContainsItem _completedquests QuestID))
  (bind _array_element (CallFunction|GetQuestActor QuestID))
  (Utilities|IsValid _array_element
    (:Is%20Valid
      (return _returnvalue (Variables|/Game/DEV/Ben_S/BPS/Quest/QuestBP.QuestBP_C|GetIsTurnedIn _array_element)))
    (:Is%20Not%20Valid
      (return _returnvalue true))))

(fn IsStageIndexEqual
  (params (Index :type Integer))
  (return (== Index (.StageNumber (Utilities|Struct|BreakDS_QuestStageDetails (Utilities|Array|Get(acopy) (.stage (Variables|Default|GetQuestDetails)) Index))))))