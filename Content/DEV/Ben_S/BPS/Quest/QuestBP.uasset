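; Quest Blueprint that tracks one quest's progress through the stages and objectives defined in the DT_QuestData table.
; On BeginPlay it loads the current stage and binds to the player character's objective ID event.
; Incoming values update a per-objective progress map, and meeting every required quantity advances the stage.
; After the last stage it marks itself complete and, if auto-complete is set, notifies the player's AC_Questlog.
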(event EventBeginPlay
  (CallFunction|GetQuestDetails)
  (bind _asbp_player_character (Utilities|Casting|CastToBP_PlayerCharacter (CallFunction|GetCharacterBP)))
  (EventDispatchers|BindEventtoOnObjectiveIDCalled _asbp_player_character (EventDispatchers|CreateEvent :!event OnObjectiveIDHeard)))

(fn ConstructionScript)

(fn OnObjectiveIDHeard
  (params (ObjectiveID :type String) (Value :type Integer))
  (bind _currentobjectiveprogress (Variables|Default|GetCurrentObjectiveProgress))
  (bind (_value _returnvalue) (Utilities|Map|Find _currentobjectiveprogress ObjectiveID))
  (if (> (Class|KismetMathLibrary|SignOfInteger Value) 0)
    (if _returnvalue
      (if (< _value (.Quantity (Utilities|Struct|BreakDS_ObjectiveDetails (CallFunction|GetObjectiveDatabyID ObjectiveID))))
        (Utilities|Map|Add (Variables|Default|GetCurrentObjectiveProgress) ObjectiveID (+ _value Value))
        (CallFunction|IsObjectiveComplete ObjectiveID)
        (Default|CallOnObjectiveHeard)
        (return))
      (else
        (return)))
    (else
      (Utilities|Map|Add (Variables|Default|GetCurrentObjectiveProgress) ObjectiveID (+ (.Value (Utilities|Map|Find (Variables|Default|GetCurrentObjectiveProgress) ObjectiveID)) Value))
      (return))))

(fn GetQuestDetails
  (bind _returnvalue (Utilities|GetDataTableRow "/Game/DEV/Ben_S/Data/DT_QuestData.DT_QuestData" (Variables|Default|GetQuestID))
    (:then
      (bind _output_get (Variables|Default|SetQuestDetails _returnvalue))
      (bind _output_get_2 (Variables|Default|SetCurrentStageDetails (Utilities|Array|Get(acopy) (.Stage (Utilities|Struct|BreakDS_QuestDetails _output_get)) (Variables|Default|GetCurrentStage))))
      (Utilities|Map|Clear (Variables|Default|GetCurrentObjectiveProgress))
      (for _array_element (.Objective (Utilities|Struct|BreakDS_QuestStageDetails _output_get_2))
        (Utilities|Map|Add (Variables|Default|GetCurrentObjectiveProgress) (.ObjectiveID (Utilities|Struct|BreakDS_ObjectiveDetails _array_element)) 0)))))

(fn GetObjectiveDatabyID
  (params (ObjectiveID :type String))
  (for _array_element (.Objective (Utilities|Struct|BreakDS_QuestStageDetails (Variables|Default|GetCurrentStageDetails)))
    (if (Utilities|Enum|Equal(Enum) (.ObjectiveID (Utilities|Struct|BreakDS_ObjectiveDetails _array_element)) ObjectiveID)
      (return _array_element))))

(fn IsObjectiveComplete
  (params (ObjectiveID :type String))
  (if (>= (.Value (Utilities|Map|Find (Variables|Default|GetCurrentObjectiveProgress) ObjectiveID)) (.Quantity (Utilities|Struct|BreakDS_ObjectiveDetails (CallFunction|GetObjectiveDatabyID ObjectiveID))))
    (bind _return (CallFunction|IsAllObjectivesComplete))
    (if _return
      (bind _result (Math|Integer|IncrementInt (Variables|Default|GetCurrentStage))
        (:%20%20
          (if (Utilities|Array|IsValidIndex (.stage (Variables|Default|GetQuestDetails)) _result)
            (CallFunction|GetQuestDetails)
            (else
              (Variables|Default|SetIsComplete true)
              (if (.autocomplete (Variables|Default|GetQuestDetails))
                (Default|CompleteQuest (Actor|GetComponentbyClass (Game|GetPlayerCharacter 0) "/Game/DEV/Ben_S/BPS/Quest/AC_Questlog.AC_Questlog_C") (Variables|Default|GetQuestID))))))))))

(fn IsAllObjectivesComplete
  (for _array_element (.Objective (Utilities|Struct|BreakDS_QuestStageDetails (Variables|Default|GetCurrentStageDetails)))
    (if (not (>= (.Value (Utilities|Map|Find (Variables|Default|GetCurrentObjectiveProgress) (.ObjectiveID (Utilities|Struct|BreakDS_ObjectiveDetails _array_element)))) (.Quantity (Utilities|Struct|BreakDS_ObjectiveDetails (CallFunction|GetObjectiveDatabyID (.ObjectiveID (Utilities|Struct|BreakDS_ObjectiveDetails _array_element)))))))
      (bind _output_get (LocalVariables|SetLocalAllComplete false))
      (return _output_get)))
  (return (LocalVariables|GetLocalAllComplete)))

(fn IsStageIndexEqual
  (params (Index :type Integer))
  (bind _questdetails (Variables|Default|GetQuestDetails))
  (for _array_element (.stage _questdetails)
    (if (== Index (Utilities|Array|FindItem :TargetArray (.stage _questdetails)))
      (return))))