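; AutoQuestBP is a quest-giver Blueprint that adds a quest to the character's questlog through its GiveQuest event; the event's trigger is not defined here.
; It queries the character's ACQuestlog and calls AddNewQuest only if the quest is neither active nor completed.
; The duplicate checks use the QuestData row name, while the quest added comes from the event's QuestID parameter.
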(event Custom|GiveQuest
  (params (QuestID :type Name))
  (bind _player (CallFunction|GetCharacterBP))
  (bind _questdata (Variables|Default|GetQuestData))
  (bind _ac_questlog (Variables|/Game/DEV/Ben_H/Blueprints/Characters/Player/BP_PlayerCharacter.BP_PlayerCharacter_C|GetAC_Questlog _player))
  (if (and (not (Default|QueryActiveQuest _ac_questlog (.rowname _questdata))) (not (.ReturnValue (Default|QueryCompletedQuests _ac_questlog (.rowname _questdata)))))
    (Default|AddNewQuest (Variables|/Game/DEV/Ben_H/Blueprints/Characters/Player/BP_PlayerCharacter.BP_PlayerCharacter_C|GetAC_Questlog (CallFunction|GetCharacterBP)) QuestID)))

(fn ConstructionScript)