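; AC_Inventory is an inventory component that keeps a map of items to quantities for the quest system.
; AddToInventory adds the quantity to the stored count, then calls the objective event on the player character with the item name as objective ID and the added quantity as value.
; QueryInventory returns the stored count for a given item.
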(event EventBeginPlay)

(event EventTick
  (params (DeltaSeconds :type Float%20%28single-precision%29)))

(fn AddtoInventory
  (params (Quantity :type Integer) (Item :type Name))
  (Utilities|Map|Add (Variables|Default|GetContent) Item (+ Quantity (.Value (Utilities|Map|Find (Variables|Default|GetContent) Item))))
  (bind _asbp_player_character (Utilities|Casting|CastToBP_PlayerCharacter (Game|GetPlayerCharacter 0)))
  (Default|CallOnObjectiveIDCalled _asbp_player_character (Utilities|String|ToString(Name) Item) Quantity))

(fn QueryInventory
  (params (Item :type Name))
  (return (.Value (Utilities|Map|Find (Variables|Default|GetContent) Item))))