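; Tree NPC that gives one of two quests based on garden-quest completion and talks once the player has the TreeInteract reward.
; Interaction ducks music, fades in a vignette and dialogue widget, and blends the camera to the NPC for conversations.
; Quest or generic lines type out letter by letter via a delayed macro loop with keyboard sounds.
; F advances conversations; finishing quest dialogue reports objective progress and restores camera, music and interaction.
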(event Custom|ReverseVignette
  (bind _dialoguebox (Variables|Default|GetDialogueBox))
  ;[0.05127 0.05127 0.05127] Regular Dialogue (Primary Interaction)
  (Utilities|FlowControl|Sequence
    (:then_0
      (bind _newtrack_0 (Timeline|Timeline_1 Reverse)
        (:Update
          (CallFunction|Vignette _newtrack_0))
        (:Finished
          (Utilities|FlowControl|DoOnce false :!label _label
            (:Completed
              (CallFunction|MoveDialogueBox)
              (bind _asbp_interact_prompt (Utilities|Casting|CastToBP_InteractPrompt (Variables|/Script/Engine.ChildActorComponent|GetChildActor (Variables|Default|GetBP_InteractPrompt))))
              (Variables|/Game/DEV/Taylor/BP_Actors/BP_InteractPrompt.BP_InteractPrompt_C|SetCanInteract? _asbp_interact_prompt false)
              (Utilities|FlowControl|Sequence
                (:then_0
                  (bind _newtrack_0_2 (Timeline|Timeline_2 Play)
                    (:Update
                      (Widget|SetRenderOpacity (Variables|/Game/DEV/Taylor/Widgets/WI_DialogueTree.WI_DialogueTree_C|GetVertBox_Text _dialoguebox) _newtrack_0_2)
                      (CallFunction|SetOutlineOpacity (Variables|/Game/DEV/Taylor/Widgets/WI_DialogueTree.WI_DialogueTree_C|GetBorder_12 _dialoguebox) _newtrack_0_2)
                      (Utilities|FlowControl|DoOnce false
                        (:Completed
                          (if (Utilities|Array|IsEmpty (Variables|Default|GetQuestDialogue))
                            (bind _finished (CallFunction|GenericDialogueText :!label _label_2))
                            (Utilities|LoopText _finished
                              (:then
                                (goto _label_2))
                              (:Finished
                                (Utilities|FlowControl|Delay 1.0)
                                (CallFunction|DialogueFinished)
                                (bind _result (Math|Integer|IncrementInt (Variables|Default|GetArrayIndex))
                                  (:%20%20
                                    (if (> _result (Utilities|Array|LastIndex (Variables|Default|GetDialogue)))
                                      (Variables|Default|SetArrayIndex 0))))))
                            (else
                              (bind _finished_2 (CallFunction|QuestDialogueText :!label _label_3))
                              (Utilities|LoopText _finished_2
                                (:then
                                  (goto _label_3))
                                (:Finished
                                  (if (Variables|Default|GetQuestDialogueConversation)
                                    (Input|EnableInput (Game|GetPlayerController 0))
                                    (Default|ShowPrompt (Variables|Default|GetDialogueBox))
                                    (else
                                      (Utilities|FlowControl|Delay 1.0)
                                      (CallFunction|DialogueFinished)
                                      (bind _result_2 (Math|Integer|IncrementInt (Variables|Default|GetQuestDialogueArrayIndex))
                                        (:%20%20
                                          (if (> _result_2 (Utilities|Array|LastIndex (Variables|Default|GetQuestDialogue)))
                                            (Variables|Default|SetQuestDialogueArrayIndex 0))
                                          (bind _asbp_tp_interface_example (Utilities|Casting|CastToBP_TP_InterfaceExample (Game|GetPlayerCharacter 0)))
                                          (Default|ObjectiveProgress _asbp_tp_interface_example (Variables|Default|GetNPCName)))))))))))))))))))))
    (:then_1
      (Utilities|FlowControl|Delay 1.1)
      (goto _label Reset))))

(event Custom|ShowDialogue
  (bind _returnvalue (Game|GetPlayerController 0))
  (bind _dialoguebox (Variables|Default|GetDialogueBox))
  ;[0.05127 0.05127 0.05127] Regular Dialogue (Primary Interaction)
  (bind _asgi_wellness_town (Utilities|Casting|CastToGI_WellnessTown (Game|GetGameInstance)))
  (Audio|Components|Audio|AdjustVolume (Variables|/Game/DEV/Taylor/GameInstance/GI_WellnessTown.GI_WellnessTown_C|GetGameMusic _asgi_wellness_town) 1.0 0.25 "Linear" :!class /Script/Engine.AudioComponent)
  (bind _asbp_tp_interface_example (Utilities|Casting|CastToBP_TP_InterfaceExample (Game|GetPlayerCharacter 0)))
  (Variables|/Game/DEV/Taylor/BP_CC/BP_TP_InterfaceExample.BP_TP_InterfaceExample_C|SetCanInteract? _asbp_tp_interface_example false)
  (if (Variables|Default|GetQuestDialogueConversation)
    (Input|DisableInput (Game|GetPlayerCharacter 0) _returnvalue)
    (Game|Player|SetViewTargetwithBlend _returnvalue self 1.0 "VTBlend_Linear" 0.0 false)
    (Variables|Default|SetVignetteIntensity 1.5)
    (bind _newtrack_0 (Timeline|Timeline_1 Play)
      (:Update
        (CallFunction|Vignette _newtrack_0))
      (:Finished
        (Utilities|FlowControl|DoOnce false
          (:Completed
            (CallFunction|MoveDialogueBox)
            (bind _asbp_interact_prompt (Utilities|Casting|CastToBP_InteractPrompt (Variables|/Script/Engine.ChildActorComponent|GetChildActor (Variables|Default|GetBP_InteractPrompt))))
            (Variables|/Game/DEV/Taylor/BP_Actors/BP_InteractPrompt.BP_InteractPrompt_C|SetCanInteract? _asbp_interact_prompt false)
            (Utilities|FlowControl|Sequence
              (:then_0
                (bind _newtrack_0_2 (Timeline|Timeline_2 Play)
                  (:Update
                    (Widget|SetRenderOpacity (Variables|/Game/DEV/Taylor/Widgets/WI_DialogueTree.WI_DialogueTree_C|GetVertBox_Text _dialoguebox) _newtrack_0_2)
                    (CallFunction|SetOutlineOpacity (Variables|/Game/DEV/Taylor/Widgets/WI_DialogueTree.WI_DialogueTree_C|GetBorder_12 _dialoguebox) _newtrack_0_2)
                    (Utilities|FlowControl|DoOnce false
                      (:Completed
                        (if (Utilities|Array|IsEmpty (Variables|Default|GetQuestDialogue))
                          (bind _finished (CallFunction|GenericDialogueText :!label _label))
                          (Utilities|LoopText _finished
                            (:then
                              (goto _label))
                            (:Finished
                              (Utilities|FlowControl|Delay 1.0)
                              (CallFunction|DialogueFinished)
                              (bind _result (Math|Integer|IncrementInt (Variables|Default|GetArrayIndex))
                                (:%20%20
                                  (if (> _result (Utilities|Array|LastIndex (Variables|Default|GetDialogue)))
                                    (Variables|Default|SetArrayIndex 0))))))
                          (else
                            (bind _finished_2 (CallFunction|QuestDialogueText :!label _label_2))
                            (Utilities|LoopText _finished_2
                              (:then
                                (goto _label_2))
                              (:Finished
                                (if (Variables|Default|GetQuestDialogueConversation)
                                  (Input|EnableInput (Game|GetPlayerController 0))
                                  (Default|ShowPrompt (Variables|Default|GetDialogueBox))
                                  (else
                                    (Utilities|FlowControl|Delay 1.0)
                                    (CallFunction|DialogueFinished)
                                    (bind _result_2 (Math|Integer|IncrementInt (Variables|Default|GetQuestDialogueArrayIndex))
                                      (:%20%20
                                        (if (> _result_2 (Utilities|Array|LastIndex (Variables|Default|GetQuestDialogue)))
                                          (Variables|Default|SetQuestDialogueArrayIndex 0))
                                        (bind _asbp_tp_interface_example_2 (Utilities|Casting|CastToBP_TP_InterfaceExample (Game|GetPlayerCharacter 0)))
                                        (Default|ObjectiveProgress _asbp_tp_interface_example_2 (Variables|Default|GetNPCName))))))))))))))))))))
    (else
      (Variables|Default|SetVignetteIntensity 1.25)
      (Timeline|Timeline_1 Play))))

(event Custom|DialogueFinished
  (bind _dialoguebox (Variables|Default|GetDialogueBox))
  ;[0.05127 0.05127 0.05127] Regular Dialogue (Primary Interaction)
  (Game|Player|SetViewTargetwithBlend (Game|GetPlayerController 0) (Game|GetPlayerCharacter 0) 1.0 "VTBlend_Linear" 0.0 false)
  (Utilities|FlowControl|Sequence
    (:then_0
      (bind _newtrack_0 (Timeline|Timeline_2 Reverse)
        (:Update
          (Widget|SetRenderOpacity (Variables|/Game/DEV/Taylor/Widgets/WI_DialogueTree.WI_DialogueTree_C|GetVertBox_Text _dialoguebox) _newtrack_0)
          (CallFunction|SetOutlineOpacity (Variables|/Game/DEV/Taylor/Widgets/WI_DialogueTree.WI_DialogueTree_C|GetBorder_12 _dialoguebox) _newtrack_0)
          (Utilities|FlowControl|DoOnce false :!label _label
            (:Completed
              (if (Utilities|Array|IsEmpty (Variables|Default|GetQuestDialogue))
                (bind _finished (CallFunction|GenericDialogueText :!label _label_2))
                (Utilities|LoopText _finished
                  (:then
                    (goto _label_2))
                  (:Finished
                    (Utilities|FlowControl|Delay 1.0)
                    (CallFunction|DialogueFinished)
                    (bind _result (Math|Integer|IncrementInt (Variables|Default|GetArrayIndex))
                      (:%20%20
                        (if (> _result (Utilities|Array|LastIndex (Variables|Default|GetDialogue)))
                          (Variables|Default|SetArrayIndex 0))))))
                (else
                  (bind _finished_2 (CallFunction|QuestDialogueText :!label _label_3))
                  (Utilities|LoopText _finished_2
                    (:then
                      (goto _label_3))
                    (:Finished
                      (if (Variables|Default|GetQuestDialogueConversation)
                        (Input|EnableInput (Game|GetPlayerController 0))
                        (Default|ShowPrompt (Variables|Default|GetDialogueBox))
                        (else
                          (Utilities|FlowControl|Delay 1.0)
                          (CallFunction|DialogueFinished)
                          (bind _result_2 (Math|Integer|IncrementInt (Variables|Default|GetQuestDialogueArrayIndex))
                            (:%20%20
                              (if (> _result_2 (Utilities|Array|LastIndex (Variables|Default|GetQuestDialogue)))
                                (Variables|Default|SetQuestDialogueArrayIndex 0))
                              (bind _asbp_tp_interface_example (Utilities|Casting|CastToBP_TP_InterfaceExample (Game|GetPlayerCharacter 0)))
                              (Default|ObjectiveProgress _asbp_tp_interface_example (Variables|Default|GetNPCName)))))))))))))))
    (:then_1
      (CallFunction|ReverseVignette)
      (bind _asgi_wellness_town (Utilities|Casting|CastToGI_WellnessTown (Game|GetGameInstance)))
      (Audio|Components|Audio|AdjustVolume (Variables|/Game/DEV/Taylor/GameInstance/GI_WellnessTown.GI_WellnessTown_C|GetGameMusic _asgi_wellness_town) 1.0 1.0 "Linear" :!class /Script/Engine.AudioComponent)
      (Utilities|FlowControl|Delay 1.1)
      (bind _asbp_tp_interface_example_2 (Utilities|Casting|CastToBP_TP_InterfaceExample (Game|GetPlayerCharacter 0)))
      (Variables|/Game/DEV/Taylor/BP_CC/BP_TP_InterfaceExample.BP_TP_InterfaceExample_C|SetCanInteract? _asbp_tp_interface_example_2 true)
      (Variables|/Game/DEV/Taylor/BP_Actors/BP_InteractPrompt.BP_InteractPrompt_C|SetCanInteract? (stale Custom|ReverseVignette _asbp_interact_prompt) true)
      (goto _label Reset))))

(event Custom|CustomEvent
  ;[0.05127 0.05127 0.05127] Secondary Interaction
  (bind _asbp_interact_prompt (Utilities|Casting|CastToBP_InteractPrompt (Variables|/Script/Engine.ChildActorComponent|GetChildActor (Variables|Default|GetBP_InteractPrompt))))
  (if (Variables|/Game/DEV/Taylor/BP_Actors/BP_InteractPrompt.BP_InteractPrompt_C|GetCanInteract? _asbp_interact_prompt)
    _))

(event EventBeginPlay
  (bind _npcname (Variables|Default|GetNPCName))
  (bind _returnvalue (Utilities|Text|ToText(String) _npcname))
  (bind _returnvalue_2 (UserInterface|CreateWidget "/Game/DEV/Taylor/Widgets/WI_DialogueTree.WI_DialogueTree_C"))
  (UserInterface|Viewport|AddtoViewport _returnvalue_2 0)
  (bind _output_get (Variables|Default|SetDialogueBox _returnvalue_2))
  (Variables|/Script/UMG.TextBlock|SetText (Variables|/Game/DEV/Taylor/Widgets/WI_DialogueTree.WI_DialogueTree_C|GetTextBlock_Name _output_get) _returnvalue)
  (Variables|/Script/UMG.TextBlock|SetText (Variables|/Game/DEV/Taylor/Widgets/WI_DialogueTree.WI_DialogueTree_C|GetTextBlock_Name_1 _output_get) _returnvalue)
  (Utilities|FlowControl|Delay 0.2)
  (bind _asgi_wellness_town (Utilities|Casting|CastToGI_WellnessTown (Game|GetGameInstance)))
  (if (Utilities|Array|ContainsItem (Variables|/Game/DEV/Taylor/GameInstance/GI_WellnessTown.GI_WellnessTown_C|GetCompletedQuests _asgi_wellness_town) "1001_CleanGarden")
    (Default|GiveQuest (Variables|Default|GetQuestGiverComponent1))
    (else
      (Default|GiveQuest (Variables|Default|GetQuestGiverComponent))))
  (Utilities|FlowControl|Delay 0.34)
  (bind _objective (Utilities|GetObjective)
    (:output
      (if (Utilities|Enum|Equal(Enum) (.ObjectiveName (Utilities|Struct|BreakS_ObjectiveDetails _objective)) (Utilities|Text|ToText(String) "Tree start"))
        (Variables|/Script/UMG.TextBlock|SetText (Variables|/Game/DEV/Taylor/Widgets/WI_DialogueTree.WI_DialogueTree_C|GetTextBlock_Name (Variables|Default|GetDialogueBox)) "????")
        (Utilities|FlowControl|Delay 5.0)
        (Variables|/Script/UMG.TextBlock|SetText (Variables|/Game/DEV/Taylor/Widgets/WI_DialogueTree.WI_DialogueTree_C|GetTextBlock_Name (Variables|Default|GetDialogueBox)) (Utilities|Text|ToText(String) (Variables|Default|GetNPCName)))))))

(event EventGeneralInteract
  ;[0.05127 0.05127 0.05127] Primary Interaction
  (bind _asbp_tp_interface_example (Utilities|Casting|CastToBP_TP_InterfaceExample (Game|GetPlayerCharacter 0)))
  (if (Utilities|Array|ContainsItem (Variables|/Game/DEV/Taylor/BP_CC/BP_TP_InterfaceExample.BP_TP_InterfaceExample_C|GetQuestRewards _asbp_tp_interface_example) "TreeInteract")
    (bind _asbp_interact_prompt (Utilities|Casting|CastToBP_InteractPrompt (Variables|/Script/Engine.ChildActorComponent|GetChildActor (Variables|Default|GetBP_InteractPrompt))))
    (if (Variables|/Game/DEV/Taylor/BP_Actors/BP_InteractPrompt.BP_InteractPrompt_C|GetCanInteract? _asbp_interact_prompt)
      (CallFunction|ShowDialogue))))

(event EventShowPrompt
  ;[0.05127 0.05127 0.05127] ButtonPrompt
  (bind _asbp_tp_interface_example (Utilities|Casting|CastToBP_TP_InterfaceExample (Game|GetPlayerCharacter 0)))
  (if (Utilities|Array|ContainsItem (Variables|/Game/DEV/Taylor/BP_CC/BP_TP_InterfaceExample.BP_TP_InterfaceExample_C|GetQuestRewards _asbp_tp_interface_example) "TreeInteract")
    (bind _asbp_interact_prompt (Utilities|Casting|CastToBP_InteractPrompt (Variables|/Script/Engine.ChildActorComponent|GetChildActor (Variables|Default|GetBP_InteractPrompt))))
    (Default|ShowPrompt _asbp_interact_prompt)))

(event Input|KeyboardEvents|F
  (params (Key :type Key%20Structure :default "None"))
  ;[0.05127 0.05127 0.05127] Continue current dialogue (E Input: located in interact prompt BP)
  (:Pressed
    (Default|HidePrompt (Variables|Default|GetDialogueBox))
    (Input|DisableInput (Game|GetPlayerController 0))
    (Variables|Default|Setletters 1)
    (bind _output_get (Variables|Default|SetQuestDialogueArrayIndex (+ (Variables|Default|GetQuestDialogueArrayIndex) 1)))
    (if (> _output_get (Utilities|Array|LastIndex (Variables|Default|GetQuestDialogue)))
      (if (Variables|Default|GetQuestDialogueConversation)
        (Variables|Default|SetQuestDialogueArrayIndex 0)
        (CallFunction|DialogueFinished)
        (bind _asbp_tp_interface_example (Utilities|Casting|CastToBP_TP_InterfaceExample (Game|GetPlayerCharacter 0)))
        (Default|ObjectiveProgress _asbp_tp_interface_example (Variables|Default|GetNPCName))
        (Utilities|FlowControl|Delay 0.1)
        (Input|EnableInput (Game|GetPlayerCharacter 0) (Game|GetPlayerController 0))
        (else
          (Variables|Default|SetQuestDialogueArrayIndex 0)))
      (else
        ;[0.05127 0.05127 0.05127] Regular Dialogue (Primary Interaction)
        (bind _finished (CallFunction|QuestDialogueText :!label _label))
        (Utilities|LoopText _finished
          (:then
            (goto _label))
          (:Finished
            (if (Variables|Default|GetQuestDialogueConversation)
              (Input|EnableInput (Game|GetPlayerController 0))
              (Default|ShowPrompt (Variables|Default|GetDialogueBox))
              (else
                (Utilities|FlowControl|Delay 1.0)
                (CallFunction|DialogueFinished)
                (bind _result (Math|Integer|IncrementInt (Variables|Default|GetQuestDialogueArrayIndex))
                  (:%20%20
                    (if (> _result (Utilities|Array|LastIndex (Variables|Default|GetQuestDialogue)))
                      (Variables|Default|SetQuestDialogueArrayIndex 0))
                    (bind _asbp_tp_interface_example_2 (Utilities|Casting|CastToBP_TP_InterfaceExample (Game|GetPlayerCharacter 0)))
                    (Default|ObjectiveProgress _asbp_tp_interface_example_2 (Variables|Default|GetNPCName))))))))))))

(fn ConstructionScript)

(fn GenericDialogueText
  (bind _dialogue (Variables|Default|GetDialogue))
  (bind _arrayindex (Variables|Default|GetArrayIndex))
  (bind _output (Utilities|Array|Get(acopy) _dialogue _arrayindex))
  (bind (_dialogueletter _letter) (Utilities|AddLetter _output (Variables|Default|Getletters))
    (:Output
      (Variables|Default|Setletters _letter)
      (Variables|/Script/UMG.MultiLineEditableTextBox|SetText (Variables|/Game/DEV/Taylor/Widgets/WI_DialogueTree.WI_DialogueTree_C|GetMultiLineEditableTextBox_349 (Variables|Default|GetDialogueBox)) (Utilities|Text|ToText(String) _dialogueletter))
      (return (>= (Utilities|String|Len _dialogueletter) (Utilities|String|Len _output))))))

(fn MoveDialogueBox
  (bind _widget (Variables|Default|GetWidget))
  (bind _widget_2 (Variables|Default|GetWidget))
  (bind _returnvalue (UserInterface|GetWidget _widget_2))
  (if (>= (.y (Transformation|GetWorldLocation (Variables|/Script/Engine.Character|GetCapsuleComponent (Game|GetPlayerCharacter 0)))) (.y (Transformation|GetWorldLocation (Variables|Default|GetDefaultSceneRoot))))
    (Transformation|SetRelativeLocation _widget (Math|Vector|MakeVector 0.0 -175.0 135.0) false false)
    (bind _aswi_dialogue (Utilities|Casting|CastToWI_Dialogue _returnvalue))
    (Variables|/Script/UMG.Widget|SetRenderTransform (Variables|/Game/DEV/Taylor/Widgets/WI_Dialogue.WI_Dialogue_C|GetCanvasPanel_344 _aswi_dialogue) (Utilities|Struct|MakeWidgetTransform "(X=0.000000,Y=0.000000)" "(X=-1.000000,Y=1.000000)" "(X=0.000000,Y=0.000000)" 1.8e+02))
    (Variables|/Script/UMG.Widget|SetRenderTransform (Variables|/Game/DEV/Taylor/Widgets/WI_Dialogue.WI_Dialogue_C|GetCanvasPanel _aswi_dialogue) (Utilities|Struct|MakeWidgetTransform "(X=0.000000,Y=0.000000)" "(X=-1.000000,Y=1.000000)" "(X=0.000000,Y=0.000000)" 1.8e+02))
    (Layout|GridSlot|SetHorizontalAlignment (Class|WidgetLayoutLibrary|SlotasVerticalBoxSlot (Variables|/Game/DEV/Taylor/Widgets/WI_Dialogue.WI_Dialogue_C|GetName_Box _aswi_dialogue)) "HAlign_Right")
    (else
      (Transformation|SetRelativeLocation _widget (Math|Vector|MakeVector 0.0 175.0 135.0) false false)
      (bind _aswi_dialogue_2 (Utilities|Casting|CastToWI_Dialogue _returnvalue))
      (Variables|/Script/UMG.Widget|SetRenderTransform (Variables|/Game/DEV/Taylor/Widgets/WI_Dialogue.WI_Dialogue_C|GetCanvasPanel_344 _aswi_dialogue_2) (Utilities|Struct|MakeWidgetTransform "(X=0.000000,Y=0.000000)" "(X=1.000000,Y=1.000000)" "(X=0.000000,Y=0.000000)" 1.8e+02))
      (Variables|/Script/UMG.Widget|SetRenderTransform (Variables|/Game/DEV/Taylor/Widgets/WI_Dialogue.WI_Dialogue_C|GetCanvasPanel _aswi_dialogue_2) (Utilities|Struct|MakeWidgetTransform "(X=0.000000,Y=0.000000)" "(X=1.000000,Y=1.000000)" "(X=0.000000,Y=0.000000)" 1.8e+02))
      (Layout|GridSlot|SetHorizontalAlignment (Class|WidgetLayoutLibrary|SlotasVerticalBoxSlot (Variables|/Game/DEV/Taylor/Widgets/WI_Dialogue.WI_Dialogue_C|GetName_Box _aswi_dialogue_2)) "HAlign_Left"))))

(fn QuestDialogueText
  (bind _questdialogue (Variables|Default|GetQuestDialogue))
  (bind _questdialoguearrayindex (Variables|Default|GetQuestDialogueArrayIndex))
  (bind _output (Utilities|Array|Get(acopy) _questdialogue _questdialoguearrayindex))
  (bind (_dialogueletter _letter) (Utilities|AddLetter _output (Variables|Default|Getletters))
    (:Output
      (Variables|Default|Setletters _letter)
      (Variables|/Script/UMG.MultiLineEditableTextBox|SetText (Variables|/Game/DEV/Taylor/Widgets/WI_DialogueTree.WI_DialogueTree_C|GetMultiLineEditableTextBox_349 (Variables|Default|GetDialogueBox)) (Utilities|Text|ToText(String) _dialogueletter))
      (return (>= (Utilities|String|Len _dialogueletter) (Utilities|String|Len _output))))))

(fn SetOutlineOpacity
  (params (Outline :type Border%20Object%20Reference) (Opacity :type Float%20%28double-precision%29))
  (bind _background (Variables|/Script/UMG.Border|GetBackground Outline))
  (Class|Border|SetBrush Outline (Utilities|Struct|MakeSlateBrush (.drawas _background) (.tiling _background) (.mirroring _background) (.imagesize _background) (.margin _background) (.tintcolor _background) (Utilities|Struct|MakeSlateBrushOutlineSettings (.cornerradii (.outlinesettings _background)) (Utilities|Struct|MakeSlateColor (Utilities|Struct|MakeLinearColor (.r (.specifiedcolor (.color (.outlinesettings _background)))) (.g (.specifiedcolor (.color (.outlinesettings _background)))) (.b (.specifiedcolor (.color (.outlinesettings _background)))) Opacity) (.coloruserule (.color (.outlinesettings _background)))) (.width (.outlinesettings _background)) (.roundingtype (.outlinesettings _background)) (.busebrushtransparency (.outlinesettings _background))) (.resourceobject _background))))

(fn Vignette
  (params (Strength :type Float%20%28double-precision%29))
  (bind _returnvalue (Actor|GetActorOfClass "/Script/Engine.PostProcessVolume"))
  (Variables|/Script/Engine.PostProcessVolume|SetSettings _returnvalue (Utilities|Struct|MakePostProcessSettings (Math|Float|Lerp 0.4 (Variables|Default|GetVignetteIntensity) Strength) (Math|Float|Lerp 0.0 1e+01 Strength))))

(fn GiveQuest
  (Default|GiveQuest (Variables|Default|GetQuestGiverComponent))
  (return (Variables|Default|GetNPCName)))